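; BP_TargetVolume is a trigger area in the VR shooting game that activates a group of targets when the player enters it.
; When its Box component begins an overlap, it confirms that player 0's pawn is a VRPawn and is the overlapping actor.
; It then calls BootTarget on every entry in TargetArray.
; A VR debug log call remains in the graph but is disconnected.
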(event OnComponentBeginOverlap(Box)
  (params (OverlappedComponent :type Primitive%20Component%20Object%20Reference) (OtherActor :type Actor%20Object%20Reference) (OtherComp :type Primitive%20Component%20Object%20Reference) (OtherBodyIndex :type Integer) (bFromSweep :type Boolean) (SweepResult :type Hit%20Result%20Structure%20%28by%20ref%29))
  ;[1 1 1] 的の起動エリアにプレイヤーが入ったら、ターゲット群を起動する処理 (VRPawn が入ったら TargetArray 内の的をすべて起動する)
  (bind _asvrpawn (Utilities|Casting|CastToVRPawn (Game|Player|GetPlayerPawn 0)))
  (if (== OtherActor (Game|Player|GetPlayerPawn 0))
    (for _array_element (Variables|Default|GetTargetArray)
      (Default|BootTarget _array_element))))

(event EventBeginPlay)

(event Collision|EventActorBeginOverlap
  (params (OtherActor :type Actor%20Object%20Reference)))

(event EventTick
  (params (DeltaSeconds :type Float%20%28single-precision%29)))

(fn ConstructionScript)