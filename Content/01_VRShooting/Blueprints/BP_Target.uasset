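; BP_Target is a VR shooting target that swings into position on a BootTarget event and changes color when damaged.
; BeginPlay pitches its Scene component to -90 degrees, and BootTarget plays a timeline that drives that pitch.
; The construction script gives the Cube a magenta dynamic material instance, which AnyDamage turns black.
; Cube hits apply damage to the other actor, not the target itself.
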(event OnComponentHit(Cube)
  (params (HitComponent :type Primitive%20Component%20Object%20Reference) (OtherActor :type Actor%20Object%20Reference) (OtherComp :type Primitive%20Component%20Object%20Reference) (NormalImpulse :type Vector :default "0, 0, 0") (Hit :type Hit%20Result%20Structure%20%28by%20ref%29))
  (Game|Damage|ApplyDamage OtherActor 1e+01 0 0))

(event Custom|BootTarget
  ;[1 1 1] Boot Animation
  (bind _float (Timeline|BootTargetTimeline Play) ; 右クリック→add custom event →
    (:Update
      (Transformation|SetRelativeRotation (Variables|Default|GetScene) (Math|Rotator|MakeRotator 0.0 _float 0.0) false false))))

(event EventBeginPlay
  (Transformation|SetRelativeRotation (Variables|Default|GetScene) "-90.000000,0.000000,0.000000" false false))

(event Collision|EventActorBeginOverlap
  (params (OtherActor :type Actor%20Object%20Reference)))

(event EventTick
  (params (DeltaSeconds :type Float%20%28single-precision%29)))

(event Game|Damage|EventAnyDamage
  (params (Damage :type Float%20%28single-precision%29) (DamageType :type Damage%20Type%20Object%20Reference) (InstigatedBy :type Controller%20Object%20Reference) (DamageCauser :type Actor%20Object%20Reference))
  ;[1 1 1] 【弾ヒット時】的の色を変更
  (Utilities|IsValid (Variables|Default|GetDM%20Cube)
    (:Is%20Valid
      (Rendering|Material|SetVectorParameterValue (Variables|Default|GetDM%20Cube) "Color" "(R=0.000000,G=0.000000,B=0.000000,A=1.000000)" :!class /Script/Engine.MaterialInstanceDynamic))))

(fn ConstructionScript
  ;[1 1 1] Cube用の Dynamic Material Instance を作成して保存
  ; ※弾ヒット時の色変更はこの MID に対して行う
  (bind _returnvalue (Rendering|Material|CreateDynamicMaterialInstance (Variables|Default|GetCube) 0 "/Game/01_VRShooting/Blueprints/M_Target.M_Target" "None" :!class /Script/Engine.PrimitiveComponent))
  (Variables|Default|SetDM%20Cube _returnvalue)
  (Rendering|Material|SetMaterial (Variables|Default|GetCube) 0 (Variables|Default|GetDM%20Cube))
  (Rendering|Material|SetVectorParameterValue (Variables|Default|GetDM%20Cube) "Color" "(R=1.000000,G=0.000000,B=1.000000,A=1.000000)" :!class /Script/Engine.MaterialInstanceDynamic))